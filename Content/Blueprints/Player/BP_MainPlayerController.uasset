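; Player controller that receives mouse, keyboard and gas mask input for the player character.
; On BeginPlay it casts player character 0 to BP_My_Player and caches the reference, which is not otherwise used here.
; Look and movement axes, plus the gas mask (Masque a Gaz) press, are each forwarded to a matching Call event, with no movement or equip logic in the controller itself.
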(event `self.ReceiveBeginPlay`
  (bind _asbp_my_player (cast `/Game/Blueprints/Player/BP_My_Player` (`GameplayStatics.GetPlayerCharacter` 0)))
  (set `self.PlayerCarachere` _asbp_my_player))

(event `InputAxis|Mouse - Look Up/Down`
  (params (AxisValue :type "Float (single-precision)"))
  ;[1 1 1] Mouse - Input
  (`self.AxisMouseUpDown` AxisValue))

(event `InputAxis|Keyboard - Forward/Backward`
  (params (AxisValue :type "Float (single-precision)"))
  ;[1 1 1] Keeyboard - Input
  (`self.KeyBoardForwardBackward` AxisValue))

(event `InputAxis|Mouse - Look Right/Left`
  (params (AxisValue :type "Float (single-precision)"))
  ;[1 1 1] Mouse - Input
  (`self.AxisMouseRightLeft` AxisValue))

(event `InputAxis|Keyboard - Right/Left`
  (params (AxisValue :type "Float (single-precision)"))
  ;[1 1 1] Keeyboard - Input
  (`self.KeyBoardRightLeft` AxisValue))

(event `InputAction|Masque a Gaz`
  (params (Key :type "Key Structure"))
  ;[1 1 1] Equipe Maque a Gaz
  (:`Pressed`
    (`self.MasqueGaz`)))

(fn `UserConstructionScript`)