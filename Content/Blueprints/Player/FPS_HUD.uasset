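; FPS player HUD that shows the crosshair and handles the pause menu.
; On BeginPlay it adds the crosshair widget and rebinds the main player controller's MenuPause dispatcher, clearing any existing bindings first.
; The pause event uses a FlipFlop to alternate between opening a newly created menu with the game paused and cursor shown, and removing it to resume play.
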(event `Pausemenu`
  (bind _returnvalue (`GameplayStatics.GetPlayerController` 0))
  ;[1 1 1] Pause Menu
  (`/Engine/EditorBlueprintResources/StandardMacros.FlipFlop`
    (:`A`
      (bind _returnvalue_2 (`|CreateWidget` "/Game/UI/Pause_Menu_Widget.Pause_Menu_Widget_C"))
      (`UserWidget.AddToViewport` _returnvalue_2 0)
      (`GameplayStatics.SetGamePaused` true)
      (set `PlayerController.bShowMouseCursor` true _returnvalue))
    (:`B`
      (`Widget.RemoveFromParent` _returnvalue_2)
      (`GameplayStatics.SetGamePaused` false)
      (set `PlayerController.bShowMouseCursor` false _returnvalue))))

(event `self.ReceiveBeginPlay`
  (`self.DefaultEchapKey`)
  (bind _returnvalue (`|CreateWidget` "/Game/UI/HUD_CrossHair.HUD_CrossHair_C"))
  (`UserWidget.AddToViewport` _returnvalue 0))

(event `DefaultEchapKey`
  (bind _mainplayercontroller (`/Game/Blueprints/Player/FuctionLibrary/BFFL_CallPLayerController.CallMainPlayerController`))
  (clear `/Game/Blueprints/Player/BP_MainPlayerController.MenuPause` _mainplayercontroller)
  (add `/Game/Blueprints/Player/BP_MainPlayerController.MenuPause` _mainplayercontroller (`|CreateDelegate` :!event `Pausemenu`)))

(fn `UserConstructionScript`)