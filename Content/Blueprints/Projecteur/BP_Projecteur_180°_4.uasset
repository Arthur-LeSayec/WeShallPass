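; Searchlight actor that sweeps its yaw along a timeline and detects the player with a cone overlap.
; On detection it stops the sweep, switches its point and spot lights to the detect color, and aims the spotlight at the player every Tick.
; After a fixed delay it restores the default color and the rotation saved at BeginPlay, and the sweep resumes.
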(event `self.ReceiveTick`
  (params (DeltaSeconds :type "Float (single-precision)"))
  (if (not (`self.IsTrigger`))
    (bind (_direction _newtrack_0) (`Timeline|Timeline_0` :!label _label)
      (:`Update`
        (`SceneComponent.K2_SetWorldRotation` (`self.DefaultSceneRoot`) (`KismetMathLibrary.MakeRotator` 0.0 0.0 _newtrack_0) false false)))
    (else
      (`|ExecutionSequence`
        (:`then_0`
          (goto _label :!via `Stop`))
        (:`then_1`
          (`SceneComponent.K2_SetWorldRotation` (`self.SpotLight`) (`KismetMathLibrary.FindLookAtRotation` (`SceneComponent.K2_GetComponentLocation` (`self.DefaultSceneRoot`)) (`SceneComponent.K2_GetComponentLocation` (`Character.CapsuleComponent` (`/Game/Blueprints/Player/FuctionLibrary/BFFL_CallPLayerController.CallMyPlayerCharactere`)))) true true))))))

(event `self.ReceiveBeginPlay`
  (set `self.DefaultSpotLightRot` (`SceneComponent.K2_GetComponentRotation` (`self.SpotLight`))))

(event `self.Cone.OnComponentBeginOverlap`
  (params (OverlappedComponent :type "PrimitiveComponent Object Reference") (OtherActor :type "Actor Object Reference") (OtherComp :type "PrimitiveComponent Object Reference") (OtherBodyIndex :type Integer) (bFromSweep :type Boolean) (SweepResult :type "HitResult Structure (by ref)"))
  (cast `/Game/Blueprints/Player/BP_My_Player` OtherActor)
  (if (not (`self.IsTrigger`))
    (set `self.IsTrigger` true)
    (`LightComponent.SetLightColor` (`self.PointLight`) (`self.Detect_Color`) true)
    (`LightComponent.SetLightColor` (`self.SpotLight`) (`self.Detect_Color`) true)
    (`KismetSystemLibrary.Delay` 5.0)
    (set `self.IsTrigger` false)
    (`SceneComponent.K2_SetWorldRotation` (`self.PointLight`) (`self.DefaultSpotLightRot`) false false)
    (`SceneComponent.K2_SetWorldRotation` (`self.SpotLight`) (`self.DefaultSpotLightRot`) false false)
    (`LightComponent.SetLightColor` (`self.PointLight`) (`self.DefaultColor`) true)
    (`LightComponent.SetLightColor` (`self.SpotLight`) (`self.DefaultColor`) true)))

(fn `UserConstructionScript`)