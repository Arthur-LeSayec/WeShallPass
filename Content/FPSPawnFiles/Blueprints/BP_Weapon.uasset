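; BP_Weapon is the player's Glock-animated hitscan gun, tracking magazine and reserve ammo.
; Fire spends a round, skips the fire montage while the player is reloading, then traces from the camera with random spread and from the muzzle to that impact point.
; Reload plays a montage, waits, then refills the magazine from the reserve.
; Traces only draw debug lines; no damage is applied.
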(event `self.Fire`
  (if (> (`self.Ammocount`) 0)
    (`self.AmmoCheck`)
    (`self.LineTrace`)))

(event `self.Reload`
  (`SkeletalMeshComponent.PlayAnimation` (`self.PrimaryWeapon`) "/Game/Animation/Weapon/Glock_Reload_anim_Montage.Glock_Reload_anim_Montage" false)
  (`KismetSystemLibrary.Delay` (`self.ReloadTime`))
  (if (> (`self.MaxAmmo`) (`self.AmmoChargeur`))
    (set `self.MaxAmmo` (- (+ (`self.MaxAmmo`) (`self.Ammocount`)) (`self.AmmoChargeur`)))
    (set `self.Ammocount` (`self.AmmoChargeur`))
    (else
      (set `self.MaxAmmo` (+ (`self.MaxAmmo`) (`self.Ammocount`)))
      (if (< (`self.MaxAmmo`) (`self.AmmoChargeur`))
        (set `self.Ammocount` (`self.MaxAmmo`))
        (set `self.MaxAmmo` 0)
        (else
          (set `self.MaxAmmo` (- (`self.MaxAmmo`) (`self.AmmoChargeur`)))
          (set `self.Ammocount` (`self.AmmoChargeur`)))))))

(fn `AmmoCheck`
  (`/Engine/EditorBlueprintResources/StandardMacros.DecrementInt` (`self.Ammocount`)
    (:`  `
      (if (not (`/Game/Blueprints/Player/BP_My_Player.IsReloading` (cast `/Game/Blueprints/Player/BP_My_Player` (`GameplayStatics.GetPlayerCharacter` 0) :!pure true)))
        (`SkeletalMeshComponent.PlayAnimation` (`self.PrimaryWeapon`) "/Game/Animation/Weapon/Glock_Fire_anim_Montage.Glock_Fire_anim_Montage" false)))))

(fn `LineTrace`
  (bind _bulletspread (`self.BulletSpread`))
  (bind _returnvalue (* _bulletspread -1.0))
  (bind _camera (`/Game/Blueprints/Player/BP_My_Player.Camera` (cast `/Game/Blueprints/Player/BP_My_Player` (`GameplayStatics.GetPlayerCharacter` 0) :!pure true)))
  (bind _returnvalue_2 (`SceneComponent.K2_GetComponentLocation` _camera))
  (bind _outhit (`KismetSystemLibrary.LineTraceSingle` :`Start` _returnvalue_2 :`End` (+ (+ (* (`SceneComponent.GetForwardVector` _camera) 20000.0) _returnvalue_2) (`KismetMathLibrary.MakeVector` (`KismetMathLibrary.RandomFloatInRange` _returnvalue _bulletspread) (`KismetMathLibrary.RandomFloatInRange` _returnvalue _bulletspread) (`KismetMathLibrary.RandomFloatInRange` _returnvalue _bulletspread))) :`TraceChannel` "TraceTypeQuery1" :`DrawDebugType` "ForDuration")) ; Camera Shot
  (`KismetSystemLibrary.LineTraceSingle` :`Start` (`SceneComponent.K2_GetComponentLocation` (`self.Muzzle`)) :`End` (`.ImpactPoint` (`GameplayStatics.BreakHitResult` _outhit)) :`TraceChannel` "TraceTypeQuery1" :`DrawDebugType` "ForDuration" :`TraceColor` (struct :`R` 1.0 :`B` 0.043706 :`A` 1.0)) ; GUN Shot
)

(fn `UserConstructionScript`
  (`parent.UserConstructionScript`)
  (set `self.MaxAmmo` 32)
  (set `self.Ammocount` 8)
  (set `self.AmmoChargeur` 8)
  (set `self.ReloadTime` 2.0)
  (set `self.BulletSpread` 175.0))